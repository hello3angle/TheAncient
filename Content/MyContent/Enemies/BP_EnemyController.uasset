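; Enemy AI controller that waits for a valid pawn, runs BT_Enemy and targets the first player pawn.
; It stores the target and start location in the Blackboard and reads attack range from the pawn.
; Looping timers act as a state machine, switching from wander to chase within alert range, then between chase and attack by attack range.
; Each switch updates the EnemyState key, with chase orienting to movement and attack focusing on the target.
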(event `CheckPawn`
  (`/Engine/EditorBlueprintResources/StandardMacros.IsValid` (`self.K2_GetPawn`) :!label _label
    (:`Is Valid`
      (`self.RunBehaviorTree` "/Game/MyContent/Enemies/AI/BT_Enemy.BT_Enemy")
      (set `self.Target` (`GameplayStatics.GetPlayerPawn` 0))
      (`self.SetBlackboardKeys`)
      (bind _enemystats (message `/Game/MyContent/Enemies/BI_EnemyInteractions.GetEnemyStats` (`self.K2_GetPawn`)))
      (set `self.Attack Range` (`.AttackRange_14_B8F721BB4A3F4CBD085329B79B4E957D` (break `/Game/MyContent/Enemies/ST_EnemyStats` _enemystats)))
      (`KismetSystemLibrary.K2_SetTimer` null "WanderCheck" (`self.CheckTime`) true))
    (:`Is Not Valid`
      (`KismetSystemLibrary.Delay` 0.1)
      (`self.CheckPawn`))))

(event `self.ReceiveBeginPlay`
  (goto _label))

(event `EnterChase`
  (bind _output_get (set `self.EnemyState` "NewEnumerator1"))
  (`BlackboardComponent.SetValueAsEnum` (`self.Blackboard`) "EnemyState" _output_get)
  (message `/Game/MyContent/Enemies/BI_EnemyInteractions.ToggleOrientRotation` (`self.K2_GetPawn`) true)
  (`self.K2_ClearFocus`))

(event `EnterAttack`
  (bind _output_get (set `self.EnemyState` "NewEnumerator2"))
  (`BlackboardComponent.SetValueAsEnum` (`self.Blackboard`) "EnemyState" _output_get)
  (message `/Game/MyContent/Enemies/BI_EnemyInteractions.ToggleOrientRotation` (`self.K2_GetPawn`) false)
  (`self.K2_SetFocus` (`self.Target`)))

(fn `AttackCheck`
  (if (> (`self.GetDistanceToTarget`) (`self.Attack Range`))
    (`self.EnterChase`)
    (`KismetSystemLibrary.K2_SetTimer` null "ChaseCheck" (`self.CheckTime`) true)
    (`KismetSystemLibrary.K2_ClearTimer` null "AttackCheck")))

(fn `ChaseCheck`
  (if (<= (`self.GetDistanceToTarget`) (`self.Attack Range`))
    (`self.EnterAttack`)
    (`KismetSystemLibrary.K2_SetTimer` null "AttackCheck" (`self.CheckTime`) true)
    (`KismetSystemLibrary.K2_ClearTimer` null "ChaseCheck")))

(fn `SetBlackboardKeys`
  (`BlackboardComponent.SetValueAsObject` (`self.Blackboard`) "Target" (`self.Target`))
  (`BlackboardComponent.SetValueAsVector` (`self.Blackboard`) "StartLoc" (`self.K2_GetActorLocation` (`self.K2_GetPawn`))))

(fn `UserConstructionScript`)

(fn `WanderCheck`
  (if (<= (`self.GetDistanceToTarget`) (`self.AlertRange`))
    (`self.EnterChase`)
    (`KismetSystemLibrary.K2_SetTimer` null "ChaseCheck" (`self.CheckTime`) true)
    (`KismetSystemLibrary.K2_ClearTimer` null "WanderCheck")))