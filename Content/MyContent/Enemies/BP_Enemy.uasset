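; Enemy character with level-based stats, a camera-facing health bar, hit reactions and an XP reward on death.
; BeginPlay links the health bar widget to itself and loads EnemyStats from LevelStats by Level.
; Damage lowers health, then either plays a hit montage or triggers death, which spawns a Niagara burst, sends level-scaled XP to the player and destroys the actor.
; It also exposes attack montage, rotation toggle and stat getters; GetEnemyTarget is empty.
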(event `self.ReceiveTick`
  (params (DeltaSeconds :type "Float (single-precision)"))
  (if (not (`self.Dead`))
    (`SceneComponent.K2_SetWorldRotation` (`self.HealthBar`) (`KismetMathLibrary.FindLookAtRotation` (`SceneComponent.K2_GetComponentLocation` (`self.HealthBar`)) (`self.K2_GetActorLocation` (`GameplayStatics.GetPlayerCameraManager` 0))) false false)))

(event `self.ReceiveBeginPlay`
  (message `/Game/MyContent/Enemies/UI/BI_WSHealthBar.SetOwnerActor` (`WidgetComponent.GetWidget` (`self.HealthBar`)) self)
  (`self.SetEnemyStats`))

(event `self.ReceiveAnyDamage`
  (params (Damage :type "Float (single-precision)") (DamageType :type "DamageType Object Reference") (InstigatedBy :type "Controller Object Reference") (DamageCauser :type "Actor Object Reference"))
  (if (not (`self.Dead`))
    (bind _outhealth (`self.SetHealth` (- (`.Health_2_0F44A6864EA9D0C178EB0B90C04A80BE` (break `/Game/MyContent/Enemies/ST_EnemyStats` (`self.EnemyStats`))) Damage)))
    (if (<= _outhealth 0.0)
      (`self.Death`)
      (else
        (`self.PlayHitReact`)))))

(event `Death`
  (bind (_returnvalue_location _returnvalue_rotation) (`KismetMathLibrary.BreakTransform` (`self.GetTransform`)))
  (set `self.Dead` true)
  (`ActorComponent.K2_DestroyComponent` (`self.HealthBar`))
  (`NiagaraFunctionLibrary.SpawnSystemAtLocation` "/Game/RPGEffects/ParticlesNiagara/StatusEffects/TeleportBurst/NS_Status_Teleport_Burst.NS_Status_Teleport_Burst" _returnvalue_location _returnvalue_rotation)
  (message `/Game/MyContent/Player/BI_PlayerInteractions.ReceiveXP` (`GameplayStatics.GetPlayerPawn` 0) (* (`self.Level`) (`self.XPValue`)))
  (`self.K2_DestroyActor`))

(event `/Game/MyContent/Enemies/BI_EnemyInteractions.ToggleOrientRotation`
  (params (OrientToMovement :type Boolean))
  (set `CharacterMovementComponent.bOrientRotationToMovement` OrientToMovement (`self.CharacterMovement`)))

(fn `BasicAttack`
  (returns (Duration :type "Float (double-precision)"))
  (bind _returnvalue (`AnimInstance.Montage_Play` (`SkeletalMeshComponent.GetAnimInstance` (`self.Mesh`)) (`self.AttackMontage`) 1.0 "Duration" 0.0 true))
  (return _returnvalue))

(fn `GetEnemyStats`
  (returns (EnemyStats :type "/Game/MyContent/Enemies/ST_EnemyStats Structure"))
  (return (`self.EnemyStats`)))

(fn `GetEnemyTarget`
  (returns (Target :type "Actor Object Reference"))
  (return null))

(fn `GetLevel`
  (returns (Level :type Integer))
  (return (`self.Level`)))

(fn `PlayHitReact`
  (returns (Duration :type "Float (double-precision)"))
  (bind _returnvalue (`AnimInstance.Montage_Play` (`SkeletalMeshComponent.GetAnimInstance` (`self.Mesh`)) (`self.HitReactMontage`) 1.0 "Duration" 0.0 true))
  (return _returnvalue))

(fn `SetEnemyStats`
  (set `self.EnemyStats` (`|GetArrayItem` (`self.LevelStats`) (- (`self.Level`) 1)))
  (return))

(fn `SetHealth`
  (params (Health :type "Float (double-precision)"))
  (returns (OutHealth :type "Float (double-precision)"))
  (bind ((`MaxHealth_10_CE4B3183483B8856BA09538A3A999C9E` _maxhealth) (`BaseDamage_11_F371E34B4BE00AAFCF88748D9CE0AA89` _basedamage) (`AttackSpeed_12_5C0B09274A8C624E708E168031A40464` _attackspeed) (`AttackRate_13_6FB35AF04594FEE87C93809EFE4A99F8` _attackrate) (`AttackRange_14_B8F721BB4A3F4CBD085329B79B4E957D` _attackrange)) (break `/Game/MyContent/Enemies/ST_EnemyStats` (`self.EnemyStats`)))
  (set `self.EnemyStats` (make `/Game/MyContent/Enemies/ST_EnemyStats` Health _maxhealth _basedamage _attackspeed _attackrate _attackrange))
  (return Health))

(fn `UserConstructionScript`)