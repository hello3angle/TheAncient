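; BP_Enemy_MeleeGrunt is a melee grunt enemy that damages actors overlapping its DamageCollision component.
; ActivateDamage and DeactivateDamage open and close the hit window by switching that collision between query-only and disabled.
; Each begin overlap applies the base damage from EnemyStats to the other actor, with no filtering, and names the grunt as damage causer.
; Construction defers to the parent class.
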(event `/Game/MyContent/Enemies/BI_EnemyInteractions.ActivateDamage`
  (`PrimitiveComponent.SetCollisionEnabled` (`self.DamageCollision`) "QueryOnly"))

(event `/Game/MyContent/Enemies/BI_EnemyInteractions.DeactivateDamage`
  (`PrimitiveComponent.SetCollisionEnabled` (`self.DamageCollision`) "NoCollision"))

(event `self.DamageCollision.OnComponentBeginOverlap`
  (params (OverlappedComponent :type "PrimitiveComponent Object Reference") (OtherActor :type "Actor Object Reference") (OtherComp :type "PrimitiveComponent Object Reference") (OtherBodyIndex :type Integer) (bFromSweep :type Boolean) (SweepResult :type "HitResult Structure (by ref)"))
  (`GameplayStatics.ApplyDamage` OtherActor (`.BaseDamage_11_F371E34B4BE00AAFCF88748D9CE0AA89` (break `/Game/MyContent/Enemies/ST_EnemyStats` (`self.EnemyStats`))) null self))

(fn `UserConstructionScript`
  (`parent.UserConstructionScript`))